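; Walk-on piano actor with eight keys that each play their own 2D note when the first-person character overlaps them, plus a reaction mini-game.
; From BeginPlay, an endless delay-driven loop highlights a random key with an emissive material and waits two seconds.
; It then checks whether the player is overlapping that key, flashes it green or red with a debug print, and restores the base material before picking again.
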(event OnComponentBeginOverlap(Key1)
  (params (OverlappedComponent :type Primitive%20Component%20Object%20Reference) (OtherActor :type Actor%20Object%20Reference) (OtherComp :type Primitive%20Component%20Object%20Reference) (OtherBodyIndex :type Integer) (bFromSweep :type Boolean) (SweepResult :type Hit%20Result%20Structure%20%28by%20ref%29))
  (Utilities|Casting|CastToBP_FirstPersonCharacter OtherActor)
  (Audio|SpawnSound2D "/Game/Piano/Piano1.Piano1" 1.0 1.0 0.0 0))

(event OnComponentBeginOverlap(Key2)
  (params (OverlappedComponent :type Primitive%20Component%20Object%20Reference) (OtherActor :type Actor%20Object%20Reference) (OtherComp :type Primitive%20Component%20Object%20Reference) (OtherBodyIndex :type Integer) (bFromSweep :type Boolean) (SweepResult :type Hit%20Result%20Structure%20%28by%20ref%29))
  (Utilities|Casting|CastToBP_FirstPersonCharacter OtherActor)
  (Audio|SpawnSound2D "/Game/Piano/Piano2.Piano2" 1.0 1.0 0.0 0))

(event OnComponentBeginOverlap(Key3)
  (params (OverlappedComponent :type Primitive%20Component%20Object%20Reference) (OtherActor :type Actor%20Object%20Reference) (OtherComp :type Primitive%20Component%20Object%20Reference) (OtherBodyIndex :type Integer) (bFromSweep :type Boolean) (SweepResult :type Hit%20Result%20Structure%20%28by%20ref%29))
  (Utilities|Casting|CastToBP_FirstPersonCharacter OtherActor)
  (Audio|SpawnSound2D "/Game/Piano/Piano3.Piano3" 1.0 1.0 0.0 0))

(event OnComponentBeginOverlap(Key4)
  (params (OverlappedComponent :type Primitive%20Component%20Object%20Reference) (OtherActor :type Actor%20Object%20Reference) (OtherComp :type Primitive%20Component%20Object%20Reference) (OtherBodyIndex :type Integer) (bFromSweep :type Boolean) (SweepResult :type Hit%20Result%20Structure%20%28by%20ref%29))
  (Utilities|Casting|CastToBP_FirstPersonCharacter OtherActor)
  (Audio|SpawnSound2D "/Game/Piano/Piano4.Piano4" 1.0 1.0 0.0 0))

(event OnComponentBeginOverlap(Key5)
  (params (OverlappedComponent :type Primitive%20Component%20Object%20Reference) (OtherActor :type Actor%20Object%20Reference) (OtherComp :type Primitive%20Component%20Object%20Reference) (OtherBodyIndex :type Integer) (bFromSweep :type Boolean) (SweepResult :type Hit%20Result%20Structure%20%28by%20ref%29))
  (Utilities|Casting|CastToBP_FirstPersonCharacter OtherActor)
  (Audio|SpawnSound2D "/Game/Piano/Piano5.Piano5" 1.0 1.0 0.0 0))

(event OnComponentBeginOverlap(Key6)
  (params (OverlappedComponent :type Primitive%20Component%20Object%20Reference) (OtherActor :type Actor%20Object%20Reference) (OtherComp :type Primitive%20Component%20Object%20Reference) (OtherBodyIndex :type Integer) (bFromSweep :type Boolean) (SweepResult :type Hit%20Result%20Structure%20%28by%20ref%29))
  (Utilities|Casting|CastToBP_FirstPersonCharacter OtherActor)
  (Audio|SpawnSound2D "/Game/Piano/Piano6.Piano6" 1.0 1.0 0.0 0))

(event OnComponentBeginOverlap(Key7)
  (params (OverlappedComponent :type Primitive%20Component%20Object%20Reference) (OtherActor :type Actor%20Object%20Reference) (OtherComp :type Primitive%20Component%20Object%20Reference) (OtherBodyIndex :type Integer) (bFromSweep :type Boolean) (SweepResult :type Hit%20Result%20Structure%20%28by%20ref%29))
  (Utilities|Casting|CastToBP_FirstPersonCharacter OtherActor)
  (Audio|SpawnSound2D "/Game/Piano/Piano7.Piano7" 1.0 1.0 0.0 0))

(event OnComponentBeginOverlap(Key8)
  (params (OverlappedComponent :type Primitive%20Component%20Object%20Reference) (OtherActor :type Actor%20Object%20Reference) (OtherComp :type Primitive%20Component%20Object%20Reference) (OtherBodyIndex :type Integer) (bFromSweep :type Boolean) (SweepResult :type Hit%20Result%20Structure%20%28by%20ref%29))
  (Utilities|Casting|CastToBP_FirstPersonCharacter OtherActor)
  (Audio|SpawnSound2D "/Game/Piano/Piano8.Piano8" 1.0 1.0 0.0 0))

(event Custom|EmissiveKeyLoop
  (Utilities|FlowControl|RetriggerableDelay 0.0 :!label _label)
  (bind _output_get (Variables|Default|SetEmmisiveKey (Utilities|Array|Get(acopy) (Variables|Default|GetKeyArray) (Math|Random|RandomIntegerinRange 0 7))))
  (Rendering|Material|SetMaterial _output_get 0 "/Game/M_EmmisiveKey.M_EmmisiveKey")
  (Utilities|FlowControl|Delay 2.0)
  (if (Collision|IsOverlappingActor (Variables|Default|GetEmmisiveKey) (Variables|Default|GetBPCharacter) :!class /Script/Engine.PrimitiveComponent)
    (Development|PrintString "Key Reached" true true "(R=0.000000,G=0.512153,B=0.062463,A=1.000000)")
    (Rendering|Material|SetMaterial _output_get 0 "/AnimationSharing/AnimSharingGreen.AnimSharingGreen")
    (Utilities|FlowControl|Delay 2.0)
    (Rendering|Material|SetMaterial _output_get 0 "/Engine/BasicShapes/BasicShapeMaterial.BasicShapeMaterial")
    (goto _label)
    (else
      (Development|PrintString "Key Not Reached" true true "(R=1.000000,G=0.119660,B=0.061527,A=1.000000)")
      (Rendering|Material|SetMaterial _output_get 0 "/AnimationSharing/AnimSharingRed.AnimSharingRed")
      (Utilities|FlowControl|Delay 2.0)
      (Rendering|Material|SetMaterial _output_get 0 "/Engine/BasicShapes/BasicShapeMaterial.BasicShapeMaterial")
      (goto _label))))

(event EventBeginPlay
  (bind _returnvalue (Actor|GetActorOfClass "/Game/FirstPerson/Blueprints/BP_FirstPersonCharacter.BP_FirstPersonCharacter_C"))
  (Variables|Default|SetBPCharacter _returnvalue)
  (Variables|Default|SetKeyArray (Utilities|Array|MakeArray (Variables|Default|GetKey2) (Variables|Default|GetKey6) (Variables|Default|GetKey7) (Variables|Default|GetKey8) (Variables|Default|GetKey3) (Variables|Default|GetKey5) (Variables|Default|GetKey4) (Variables|Default|GetKey1)))
  (CallFunction|EmissiveKeyLoop))

(fn ConstructionScript)